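; BP_Projectile is a shot that resolves hits on enemies, the player and physics objects.
; Enemy hits apply the player's damage per shot, award score unless already dead, and always stun.
; Player hits not instigated by the player apply the owning enemy's damage, deduct score, launch and stun.
; These hits and velocity-scaled impulses on simulating objects spawn an effect and destroy the projectile; other hits do nothing.
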(event `self.ReceiveBeginPlay`
  ;[1 1 1] Set Player Reference
  (bind _asbp_first_person_character (cast `/Game/EHT01/Blueprints/BP_FirstPersonCharacter` (`GameplayStatics.GetPlayerPawn` 0)))
  (set `self.PlayerRef` _asbp_first_person_character))

(event `self.ReceiveHit`
  (params (MyComp :type "PrimitiveComponent Object Reference") (Other :type "Actor Object Reference") (OtherComp :type "PrimitiveComponent Object Reference") (bSelfMoved :type Boolean) (HitLocation :type "Vector Structure") (HitNormal :type "Vector Structure") (NormalImpulse :type "Vector Structure") (Hit :type "HitResult Structure (by ref)"))
  ;[1 1 1] Handles Damage and impulse to player and objects
  (bind _asbp_enemy (cast `/Game/EHT01/Blueprints/BP_Enemy` Other)
    (:`then`
      (`self.DamageEnemy` _asbp_enemy)
      (`/Game/EHT01/Blueprints/BP_Enemy.Start Stun` (`self. BPEnemyRef`))
      (`GameplayStatics.SpawnEmitterAtLocation` "/Game/Effects/ParticleSystems/Weapons/AssaultRifle/Impacts/ShotHit.ShotHit" (`self.K2_GetActorLocation`) :!label _label)
      (`self.K2_DestroyActor`) ; Then destroy this projectile
    )
    (:`CastFailed`
      (cast `/Game/EHT01/Blueprints/BP_FirstPersonCharacter` Other
        (:`then`
          (`self.DamagePlayer`)
          (goto _label))
        (:`CastFailed`
          (if (`SceneComponent.IsSimulatingPhysics` OtherComp "None")
            (`PrimitiveComponent.AddImpulseAtLocation` OtherComp (* (`self.GetVelocity`) 50.0) (0.0 0.0 0.0) "None")
            (goto _label)))))))

(fn `DamageEnemy`
  (params (` BPEnemyRef` :type "/Game/EHT01/Blueprints/BP_Enemy Object Reference"))
  (bind _output_get (set `self. BPEnemyRef` ` BPEnemyRef`))
  (if (not (`/Game/EHT01/Blueprints/BP_Enemy.IsDead` _output_get))
    (`/Game/EHT01/Blueprints/BP_Enemy.UpdateHealth` (`self. BPEnemyRef`) (`/Game/EHT01/Blueprints/BP_FirstPersonCharacter.DamagePerShot` (`self.PlayerRef`)))
    (`/Game/EHT01/Blueprints/BP_FirstPersonCharacter.IncreaseScore` (`self.PlayerRef`) (`/Game/EHT01/Blueprints/BP_Enemy.EnemyScorePerHit` (`self. BPEnemyRef`)))))

(fn `DamagePlayer`
  (if (!= (`self.Instigator`) (`self.PlayerRef`))
    (`/Game/EHT01/Blueprints/BP_FirstPersonCharacter.TakeDamage` (`self.PlayerRef`) (`/Game/EHT01/Blueprints/BP_Enemy.DamagePerShot` (cast `/Game/EHT01/Blueprints/BP_Enemy` (`self.GetOwner` self) :!pure true)))
    (`/Game/EHT01/Blueprints/BP_FirstPersonCharacter.DecreaseScore` (`self.PlayerRef`) 5)
    (`Character.LaunchCharacter` (`self.PlayerRef`) (/ (`self.GetVelocity`) 2.0) false false)
    (`/Game/EHT01/Blueprints/BP_FirstPersonCharacter.StartStun` (`self.PlayerRef`))))

(fn `UserConstructionScript`)