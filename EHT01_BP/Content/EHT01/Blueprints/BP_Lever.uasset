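; BP_Lever is an interactable lever that toggles every BP_Enemy between the normal and glowing dummy material.
; It binds ActivateLever to the first-person character's interact event on BeginPlay, while overlap begin and end enable or disable that character's interaction mode.
; Each activation plays or reverses a timeline, which offsets the lever mesh along world X from the actor's starting location, and flips IsOnEnd.
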(event `MoveLeverRight`
  ;[1 1 1] Lever movement
  (bind (_direction _levermoviment) (`Timeline|LeverTimeline` :`NewTime` (`GameplayStatics.GetWorldDeltaSeconds`) :!via `PlayFromStart` :!label _label)
    (:`Update`
      (`self.UpdateLeverLocation` _levermoviment))))

(event `MoveLeverLeft`
  ;[1 1 1] Lever movement
  (goto _label :!via `Reverse`))

(event `self.ReceiveBeginPlay`
  ;[1 1 1] Setting Variables and binding events
  (bind _asbp_first_person_character (cast `/Game/EHT01/Blueprints/BP_FirstPersonCharacter` (`GameplayStatics.GetPlayerPawn` 0)))
  (bind _output_get (set `self.PlayerRef` _asbp_first_person_character))
  (add `/Game/EHT01/Blueprints/BP_FirstPersonCharacter.InteractWithObject` _output_get (delegate `ActivateLever`))
  (set `self.LeverInitialPositon` (`self.K2_GetActorLocation` self)))

(event `ActivateLever`
  ;[1 1 1] Lever Activation Event
  (if (`self.IsOnEnd`)
    (`self.MoveLeverLeft`)
    (set `self.IsOnEnd` false)
    (bind _outactors (`GameplayStatics.GetAllActorsOfClass` "/Game/EHT01/Blueprints/BP_Enemy.BP_Enemy_C"))
    (for _array_element _outactors
      (`PrimitiveComponent.SetMaterial` (`/Game/EHT01/Blueprints/BP_Enemy.StaticMesh` _array_element) 0 "/Game/EnemyDummy/M_EnemyDummy.M_EnemyDummy"))
    (else
      (`self.MoveLeverRight`)
      (set `self.IsOnEnd` true)
      (bind _outactors_2 (`GameplayStatics.GetAllActorsOfClass` "/Game/EHT01/Blueprints/BP_Enemy.BP_Enemy_C"))
      (for _array_element_2 _outactors_2
        (`PrimitiveComponent.SetMaterial` (`/Game/EHT01/Blueprints/BP_Enemy.StaticMesh` _array_element_2) 0 "/Game/EnemyDummy/M_EnemyDummyGlow.M_EnemyDummyGlow")))))

(event `self.ReceiveActorBeginOverlap`
  (params (OtherActor :type "Actor Object Reference"))
  ;[1 1 1] Start interaction mode with player when overlapped
  (bind _asbp_first_person_character (cast `/Game/EHT01/Blueprints/BP_FirstPersonCharacter` OtherActor))
  (`/Game/EHT01/Blueprints/BP_FirstPersonCharacter.EnableInteraction` _asbp_first_person_character))

(event `self.ReceiveActorEndOverlap`
  (params (OtherActor :type "Actor Object Reference"))
  ;[1 1 1] end Interaction mode with player when overlap ends
  (bind _asbp_first_person_character (cast `/Game/EHT01/Blueprints/BP_FirstPersonCharacter` OtherActor))
  (`/Game/EHT01/Blueprints/BP_FirstPersonCharacter.DisableInteraction` _asbp_first_person_character))

(fn `UpdateLeverLocation`
  (params (X :type "Float (double-precision)"))
  (bind _output_get (set `self.LeverNewLocation` (`self.LeverInitialPositon`)))
  (bind _output_get_2 (set `self.LeverNewLocation` (`KismetMathLibrary.MakeVector` (+ (.x _output_get) X) (.y _output_get) (.z _output_get))))
  (`SceneComponent.K2_SetWorldLocation` (`self.Lever`) _output_get_2 false false))

(fn `UserConstructionScript`)