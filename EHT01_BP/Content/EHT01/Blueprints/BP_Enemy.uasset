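; Enemy shooter that turns to face the first-person player and fires BP_Projectile from its weapon's Muzzle socket on a looping timer.
; Tracking interpolates pitch and yaw through a self-calling Delay loop instead of Tick.
; UpdateHealth leads to Die, which stops firing and tilts the weapon.
; Stun blocks firing and damage until a timer ends it, then grants stun immunity until a second timer, started alongside the first, expires.
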(event `self.ReceiveBeginPlay`
  ;[1 1 1] Start Firing
  (bind _asbp_first_person_character (cast `/Game/EHT01/Blueprints/BP_FirstPersonCharacter` (`GameplayStatics.GetPlayerPawn` 0)))
  (set `self.PlayerRef` _asbp_first_person_character)
  (`self.FacePlayer`)
  (`KismetSystemLibrary.K2_SetTimer` null "Fire" (`self.FireRate`) true))

(event `FacePlayer`
  (bind (_returnvalue_roll _returnvalue_pitch _returnvalue_yaw) (`KismetMathLibrary.BreakRotator` (`KismetMathLibrary.RInterpTo` (`self.K2_GetActorRotation`) (`KismetMathLibrary.FindLookAtRotation` (`self.K2_GetActorLocation`) (`self.K2_GetActorLocation` (`self.PlayerRef`))) (`GameplayStatics.GetWorldDeltaSeconds`) (`self.TurnRate`))))
  ;[1 1 1] Face Player
  (if (`self.IsTrackingPlayer`)
    (if (not (`self.IsDead`))
      (`self.K2_SetActorRotation` (`KismetMathLibrary.MakeRotator` 0.0 _returnvalue_pitch _returnvalue_yaw))
      (`KismetSystemLibrary.Delay` 0.001)
      (`self.FacePlayer`))))

(fn `Die`
  (set `self.IsDead` true)
  (set `self.CanFire` false)
  (`SceneComponent.K2_AddLocalRotation` (`self.WeaponMesh`) (struct :`Roll` 50.0) false false))

(fn `DisableStunInvulnerability`
  (set `self.IsInvunerableToStun` false))

(fn `EndStun`
  (set `self.IsStunned` false)
  (set `self.IsInvunerableToStun` true)
  (set `self.CanTakeDamage` true)
  (if (not (`self.IsDead`))
    (set `self.CanFire` true)))

(fn `Fire`
  (bind (_returnvalue_location _returnvalue_rotation _returnvalue_scale) (`KismetMathLibrary.BreakTransform` (`SceneComponent.GetSocketTransform` (`self.WeaponMesh`) "Muzzle" "RTS_World")))
  (if (not (`self.IsStunned`))
    (if (`self.CanFire`)
      (`|SpawnActorFromClass` "/Game/EHT01/Blueprints/BP_Projectile.BP_Projectile_C" (`KismetMathLibrary.MakeTransform` _returnvalue_location _returnvalue_rotation _returnvalue_scale) "Undefined" "OverrideRootScale" self null)
      (`GameplayStatics.PlaySound2D` "/Game/FPWeapon/Audio/FirstPersonTemplateWeaponFire02.FirstPersonTemplateWeaponFire02" 1.0 1.0 0.0 null null))))

(fn `SetStunInvulnerabilityTime`
  (`KismetSystemLibrary.K2_SetTimer` null "DisableStunInvulnerability" (`self.StunInvulnerabilityTime`)))

(fn `Start Stun`
  (if (not (`self.IsStunned`))
    (if (not (`self.IsInvunerableToStun`))
      (set `self.IsStunned` true)
      (set `self.CanFire` false)
      (set `self.CanTakeDamage` false)
      (`KismetSystemLibrary.K2_SetTimer` null "EndStun" (`self.StunTime`))
      (`self.SetStunInvulnerabilityTime`))))

(fn `UpdateHealth`
  (params (Damage :type "Float (double-precision)"))
  (bind _currenthealth (`self.CurrentHealth`))
  (if (`self.CanTakeDamage`)
    (set `self.CurrentHealth` (- _currenthealth Damage))
    (if (<= _currenthealth 0.0)
      (`self.Die`))))

(fn `UserConstructionScript`)